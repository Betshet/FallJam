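; Inventory component for characters that stores picked-up items as an array of pickup info structs holding a pickup type and actor class.
; Functions add entries, check fullness against InventorySpace, and remove the first match of a type, all matches, or everything.
; Removing all of a type iterates over a copy of the array and returns the count removed.
; Adding does not check capacity itself.
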(fn AddtoInventory
  (params (PickupType :type E_PickupType%20Enum :default "NewEnumerator0") (PickupActorClass :type BP%20Pickup%20Base%20Class%20Reference))
  (Utilities|Array|Add (Variables|Default|GetInventory) (Utilities|Struct|MakeS_PickupInfo PickupType PickupActorClass))
  (return))

(fn IsInventoryFull
  (return (>= (Utilities|Array|Length (Variables|Default|GetInventory)) (Variables|Default|GetInventorySpace))))

(fn RemovefromInventory
  (params (TypeToRemove :type E_PickupType%20Enum :default "NewEnumerator0"))
  (for _array_element (Variables|Default|GetInventory)
    (if (Utilities|Enum|Equal(Enum) (.PickupType (Utilities|Struct|BreakS_PickupInfo _array_element)) TypeToRemove)
      (Utilities|Array|RemoveItem (Variables|Default|GetInventory) _array_element)
      (return))))

(fn RemoveAllItemsOfType
  (params (Type :type E_PickupType%20Enum :default "NewEnumerator0"))
  (LocalVariables|SetInventoryCopy (Variables|Default|GetInventory))
  (for _array_element (LocalVariables|GetInventoryCopy)
    (if (Utilities|Enum|Equal(Enum) (.PickupType (Utilities|Struct|BreakS_PickupInfo _array_element)) Type)
      (Math|Integer|IncrementInt (LocalVariables|GetNumberRemoved)
        (:%20%20
          (Utilities|Array|RemoveItem (Variables|Default|GetInventory) _array_element)))))
  (return (LocalVariables|GetNumberRemoved)))

(fn RemoveAllItems
  (Utilities|Array|Clear (Variables|Default|GetInventory)))