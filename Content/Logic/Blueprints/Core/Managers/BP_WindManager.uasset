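; Wind manager that runs storms which drain heat via BP_HeatManager, pausing on hub entry and resuming on exit.
; A looping timer builds wind to max, firing a one-time warning at a threshold, then further timers run the storm's duration and per-second heat drain.
; Wind changes broadcast payload events and drive player-attached Niagara leaves and wind ambience through a curve.
; Tick prints wind and storm debug text.
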(event OnEventInvoked(EnterHubListener)
  (CallFunction|StopStorm))

(event OnEventInvoked(ExitHubListener)
  (CallFunction|StartStormwithCooldown))

(event EventStart
  (CallFunction|StartStormwithCooldown)
  (CallFunction|SetUpVFX))

(event EventTick
  (params (DeltaSeconds :type Float%20%28single-precision%29))
  (Development|PrintText (Utilities|Text|FormatText "CurrentWindValue: {cWind}/{mWind} 
Storm Started:{sStarted} 
Storm Time Left: {stl}" (Variables|Default|GetCurrentWind) (Variables|Default|GetMaxWind) (Variables|Default|GetStormStarted?) (.TimeRemaining (CallFunction|GetStormTimeRemaining))) true true "(R=0.000000,G=0.660000,B=1.000000,A=1.000000)" 2.0 "wind"))

(fn ConstructionScript)

(fn StartStormwithCooldown
  (bind _returnvalue (Utilities|Time|SetTimerbyEvent (EventDispatchers|CreateEvent :!event IncrementWindValue) 1.0 true))
  (Variables|Timers|SetWindBuildupTimer _returnvalue))

(fn StartStormImmediately
  (Variables|Default|SetCurrentWind (Variables|Default|GetMaxWind))
  (Default|CallOnWindValueChanged)
  (Variables|Default|SetStormStarted? true)
  (bind _returnvalue (Utilities|Time|SetTimerbyEvent (EventDispatchers|CreateEvent :!event StopStormandAutoRestart) (Variables|Timings|GetStormDuration)))
  (Variables|Timers|SetStopStormTimer _returnvalue)
  (bind _returnvalue_2 (Utilities|Time|SetTimerbyEvent (EventDispatchers|CreateEvent :!event StormTick) 1.0 true))
  (Variables|Timers|SetStormTickTimer _returnvalue_2)
  (Effects|Components|ParticleSystem|SetFloatParameter (Variables|Default|GetAmbientVFX) "LeafSpawnRate" (Variables|VFX|GetStormLeafSpawnRate))
  (Effects|Components|ParticleSystem|SetFloatParameter (Variables|Default|GetAmbientVFX) "WindLinesSpawnRate" (Variables|VFX|GetStormWindLinesSpawnRate)))

(fn StopStorm
  (CallFunction|ChangeWindValue 0.0)
  (Default|CallOnWindValueChanged)
  (Utilities|Time|ClearandInvalidateTimerbyHandle (Variables|Timers|GetWindBuildupTimer))
  (Utilities|Time|ClearandInvalidateTimerbyHandle (Variables|Timers|GetStopStormTimer))
  (Utilities|Time|ClearandInvalidateTimerbyHandle (Variables|Timers|GetStormTickTimer))
  (Variables|Default|SetStormStarted? false)
  (Variables|Default|SetWarningGiven false)
  (Effects|Components|ParticleSystem|SetFloatParameter (Variables|Default|GetAmbientVFX) "LeafSpawnRate" (Variables|VFX|GetBaseLeafSpawnRate))
  (Effects|Components|ParticleSystem|SetFloatParameter (Variables|Default|GetAmbientVFX) "WindLinesSpawnRate" 0.0))

(fn StopStormandAutoRestart
  (CallFunction|StopStorm)
  (CallFunction|StartStormwithCooldown))

(fn IncrementWindValue
  (CallFunction|ChangeWindValue (+ (Variables|Default|GetCurrentWind) (/ (Variables|Default|GetMaxWind) (Variables|Timings|GetCooldownPeriod))))
  (if (>= (Variables|Default|GetCurrentWind) (Variables|Timings|GetStormWarningTreshold))
    (CallFunction|StormWarning))
  (if (>= (Variables|Default|GetCurrentWind) (Variables|Default|GetMaxWind))
    (Utilities|Time|ClearandInvalidateTimerbyHandle (Variables|Timers|GetWindBuildupTimer))
    (CallFunction|StartStormImmediately)))

(fn StormTick
  (bind _returnvalue (Actor|GetActorOfClass "/Game/Logic/Blueprints/Core/Managers/BP_HeatManager.BP_HeatManager_C"))
  (Default|ChangeHeat _returnvalue (* (Variables|Timings|GetHeatSapPerSecond) -1.0)))

(fn GetStormTimeRemaining
  (bind _stopstormtimer (Variables|Timers|GetStopStormTimer))
  (return (Utilities|Time|IsTimerActivebyHandle _stopstormtimer) (Utilities|Time|GetTimerRemainingTimebyHandle _stopstormtimer)))

(fn StormWarning
  (if (not (Variables|Default|GetWarningGiven))
    (Development|PrintString "WARNING: WIND IMMINENT")
    (Class|ESEvent|Invoke "/Game/Logic/Blueprints/Events/Event_OnStormWarning.Event_OnStormWarning")
    (Variables|Default|SetWarningGiven true)))

(fn ChangeWindValue
  (params (NewValue :type Float%20%28double-precision%29))
  (|InvokeEventPayload "/Game/Logic/Blueprints/Events/Event_OnWindValueChanged.Event_OnWindValueChanged" "/Game/Logic/Blueprints/Events/Payloads/Payload_WindValueChanged.Payload_WindValueChanged_C" (Variables|Default|GetCurrentWind) NewValue)
  (Variables|Default|SetCurrentWind NewValue)
  (Effects|Components|ParticleSystem|SetFloatParameter (Variables|Default|GetAmbientVFX) "WindStrength" (Math|Float|Max(Float) (* (Variables|VFX|GetStormLeafSpeed) (Math|Curves|GetFloatValue (Variables|VFX|GetWindVFXCurve) (Variables|Default|GetCurrentWind))) (Variables|VFX|GetBaseLeafSpeed)))
  (Audio|Parameter|SetFloatParameter (Variables|Default|GetWindAmbience) "WindStrength" (* (Math|Curves|GetFloatValue (Variables|VFX|GetWindVFXCurve) (Variables|Default|GetCurrentWind)) (Variables|Default|GetWarningGiven)) :!class /Script/AudioExtensions.AudioParameterControllerInterface))

(fn SetUpVFX
  (bind _returnvalue (Niagara|SpawnSystemAttached "/Game/Art/VFX/Ambient/NS_AmbientLeavesAndWind.NS_AmbientLeavesAndWind" (Variables|/Script/Engine.Actor|GetRootComponent (Game|Player|GetPlayerPawn 0)) "None" "-1500.000000,1000.000000,500.000000" "0, 0, 0" "SnapToTarget" false))
  (Variables|Default|SetAmbientVFX _returnvalue)
  (Effects|Components|ParticleSystem|SetFloatParameter (Variables|Default|GetAmbientVFX) "LeafSpawnRate" (Variables|VFX|GetBaseLeafSpawnRate))
  (Effects|Components|ParticleSystem|SetFloatParameter (Variables|Default|GetAmbientVFX) "WindStrength" (Variables|VFX|GetBaseLeafSpeed)))