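; BP_HeatManager tracks the player's heat, which can drop only outside shelters and the hub and regenerates inside them.
; Listeners for entering or leaving either place toggle regen and loss flags, and a player faint refills heat to max.
; ChangeHeat clamps the value and broadcasts an OnHeatChanged payload event.
; A looping one-second timer is started on BeginPlay, and Tick prints current heat as debug text.
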(event OnEventInvoked(EnterShelterListener)
  (Variables|Default|SetShouldRegenHeat? true)
  (Variables|Default|SetCanLoseHeat? false))

(event OnEventInvoked(LeaveShelterListener)
  (Variables|Default|SetShouldRegenHeat? false)
  (Variables|Default|SetCanLoseHeat? true))

(event OnEventInvoked(EnterHubListener)
  (Variables|Default|SetShouldRegenHeat? true)
  (Variables|Default|SetCanLoseHeat? false))

(event OnEventInvoked(ExitHubListener)
  (Variables|Default|SetShouldRegenHeat? false)
  (Variables|Default|SetCanLoseHeat? true))

(event OnEventInvoked(PlayerFaintListener)
  (CallFunction|ChangeHeat (- (Variables|Default|GetMaxHeat) (Variables|Default|GetCurrentHeat))))

(event EventTick
  (params (DeltaSeconds :type Float%20%28single-precision%29))
  (Development|PrintText (Utilities|Text|FormatText "HEAT: {c}/{m}" (Variables|Default|GetCurrentHeat) (Variables|Default|GetMaxHeat)) true true "(R=1.000000,G=0.301206,B=0.000000,A=1.000000)" 2.0 "heat"))

(event EventBeginPlay
  (CallFunction|Start))

(event EventStart
  (Utilities|Time|SetTimerbyEvent (EventDispatchers|CreateEvent :!event HeatRegenTick) 1.0 true))

(fn ConstructionScript)

(fn ChangeHeat
  (params (DeltaHeat :type Float%20%28double-precision%29))
  (LocalVariables|SetPrevHeat (Variables|Default|GetCurrentHeat))
  (if (< DeltaHeat 0.0)
    (if (Variables|Default|GetCanLoseHeat?)
      (Variables|Default|SetCurrentHeat (Math|Float|Clamp(Float) (+ DeltaHeat (Variables|Default|GetCurrentHeat)) 0.0 (Variables|Default|GetMaxHeat)) :!label _label)
      (|InvokeEventPayload "/Game/Logic/Blueprints/Events/Event_OnHeatChanged.Event_OnHeatChanged" "/Game/Logic/Blueprints/Events/Payloads/Payload_OnHeatChanged.Payload_OnHeatChanged_C" (LocalVariables|GetPrevHeat) (Variables|Default|GetCurrentHeat) DeltaHeat))
    (else
      (goto _label))))

(fn HeatDepleted
  (Development|PrintString "Heat is gone"))

(fn HeatRegenTick
  (if (Variables|Default|GetShouldRegenHeat?)
    (CallFunction|ChangeHeat (Variables|Default|GetHeatRegenPerSecond))))