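; Main menu game mode that shows the menu widget on screen and handles starting and quitting the game.
; On BeginPlay it creates the main menu widget, stores it, adds it to the viewport and binds click events to the inner buttons of its Start and Quit button widgets.
; Start opens TestMap by object reference, and Quit exits the game.
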(event Custom|OnClicked_Event
  (Game|OpenLevel(byObjectReference) "/Game/Logic/Maps/TestMap.TestMap"))

(event Custom|OnClicked_Event_0
  (Game|QuitGame 0 "Quit" false))

(event EventBeginPlay
  (bind _returnvalue (UserInterface|CreateWidget "/Game/Logic/Blueprints/Widgets/Widget_MainMenu.Widget_MainMenu_C"))
  (bind _output_get (Variables|Default|SetMainMenuWidget _returnvalue))
  (UserInterface|Viewport|AddtoViewport _output_get 0)
  (Utilities|FlowControl|Sequence
    (:then_0
      (EventDispatchers|AssignOnClicked (Variables|/Game/Logic/Blueprints/Widgets/Widget_MenuButton.Widget_MenuButton_C|GetButton_23 (Variables|/Game/Logic/Blueprints/Widgets/Widget_MainMenu.Widget_MainMenu_C|GetStartButton (Variables|Default|GetMainMenuWidget))) (delegate Custom|OnClicked_Event))
      (EventDispatchers|AssignOnClicked (Variables|/Game/Logic/Blueprints/Widgets/Widget_MenuButton.Widget_MenuButton_C|GetButton_23 (Variables|/Game/Logic/Blueprints/Widgets/Widget_MainMenu.Widget_MainMenu_C|GetQuitButton (Variables|Default|GetMainMenuWidget))) (delegate Custom|OnClicked_Event_0)))))

(fn ConstructionScript)