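; BP_Shelter is an interactable 2D shelter that toggles between empty and occupied each time Interact fires.
; Occupying or emptying it sets the Occupied flag, swaps the Paper2D flipbook and invokes the matching enter or leave event.
; While occupied, it pushes a muffling sound mix with a class override on the target sounds, then pops the mix on leaving.
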(event EventBeginPlay
  (|CallParentFunction) ; This node is disabled and will not be called.\nDrag off pins to build functionality.
)

(event Collision|EventActorBeginOverlap
  (params (OtherActor :type Actor%20Object%20Reference))
  (|CallParentFunction OtherActor) ; This node is disabled and will not be called.\nDrag off pins to build functionality.
)

(event EventTick
  (params (DeltaSeconds :type Float%20%28single-precision%29))
  (|CallParentFunction DeltaSeconds) ; This node is disabled and will not be called.\nDrag off pins to build functionality.
)

(event EventInteract
  (if (Variables|Default|GetOccupied?)
    (CallFunction|EmptyShelter)
    (else
      (CallFunction|OccupyShelter))))

(fn ConstructionScript
  (|CallParentFunction)
  (Sprite|SetFlipbook (Variables|Default|GetPaperFlipbook) (Variables|Default|GetEmptyFlipbook)))

(fn OccupyShelter
  (Class|ESEvent|Invoke "/Game/Logic/Blueprints/Events/Event_OnEnterShelter.Event_OnEnterShelter")
  (Variables|Default|SetOccupied? true)
  (Sprite|SetFlipbook (Variables|Default|GetPaperFlipbook) (Variables|Default|GetOccupiedFlipbook))
  (Audio|SetSoundMixClassOverride "/Game/Audio/Mixes/Mix_Muffled.Mix_Muffled" "/Game/Audio/Classes/MuffleTargets.MuffleTargets" 1.0 1.0 1.0 true)
  (Audio|PushSoundMixModifier "/Game/Audio/Mixes/Mix_Muffled.Mix_Muffled"))

(fn EmptyShelter
  (Class|ESEvent|Invoke "/Game/Logic/Blueprints/Events/Event_OnLeaveShelter.Event_OnLeaveShelter")
  (Variables|Default|SetOccupied? false)
  (Sprite|SetFlipbook (Variables|Default|GetPaperFlipbook) (Variables|Default|GetEmptyFlipbook))
  (Audio|PopSoundMixModifier "/Game/Audio/Mixes/Mix_Muffled.Mix_Muffled"))