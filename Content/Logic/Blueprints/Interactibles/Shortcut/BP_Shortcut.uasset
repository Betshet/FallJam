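; BP_Shortcut is an interactible shortcut that starts blocked and is permanently opened when the player interacts with it.
; Interact clears the Locked flag immediately, fades the player character out, waits briefly, calls Unlock, then fades back in, so the change happens during the fade.
; Unlock swaps the Paper2D sprite to its unblocked version, clears and hides the interaction prompt, and disables collision.
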(event EventBeginPlay
  (|CallParentFunction) ; This node is disabled and will not be called.\nDrag off pins to build functionality.
)

(event Collision|EventActorBeginOverlap
  (params (OtherActor :type Actor%20Object%20Reference))
  (|CallParentFunction OtherActor) ; This node is disabled and will not be called.\nDrag off pins to build functionality.
)

(event EventTick
  (params (DeltaSeconds :type Float%20%28single-precision%29))
  (|CallParentFunction DeltaSeconds) ; This node is disabled and will not be called.\nDrag off pins to build functionality.
)

(event EventInteract
  (if (Variables|Default|GetLocked?)
    (Variables|Default|SetLocked? false)
    (bind _asbp_top_down_character (Utilities|Casting|CastToBP_TopDownCharacter (Game|Player|GetPlayerPawn 0)))
    (Default|FadeOut _asbp_top_down_character)
    (Utilities|FlowControl|Delay 1.0)
    (CallFunction|Unlock)
    (Default|FadeinAfterDelay _asbp_top_down_character)))

(fn ConstructionScript
  (Rendering|Components|Sprite|SetSprite (Variables|Default|GetPaperSprite) (Variables|Default|GetBlockedSprite))
  (|CallParentFunction))

(fn Unlock
  (bind _interactionprompt (Variables|Default|GetInteractionPrompt))
  (Rendering|Components|Sprite|SetSprite (Variables|Default|GetPaperSprite) (Variables|Default|GetUnBlockedSprite))
  (Variables|Default|SetLocked? false)
  (UserInterface|SetWidget _interactionprompt 0)
  (Rendering|SetVisibility _interactionprompt false false)
  (Collision|SetCollisionEnabled (Variables|Default|GetCollisions) "NoCollision"))