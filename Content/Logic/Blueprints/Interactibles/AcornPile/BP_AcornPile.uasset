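; Interactable acorn pile that collects the player's acorns and ends the game once it is full.
; On interact, it removes all items of one pickup type from the player's inventory, found through the game mode, and adds the same count to its own inventory component.
; When none are handed over, it briefly shows a thought bubble on a timer.
; A full pile fades the player out and opens the end-game map after a short delay.
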(event Custom|HideBubble
  (Rendering|SetVisibility (Variables|Default|GetThoughtBubble) false true))

(event Custom|ShowBubble
  (Rendering|SetVisibility (Variables|Default|GetThoughtBubble) true true)
  (Utilities|Time|SetTimerbyEvent (delegate Custom|HideBubble) 3.0))

(event Custom|EndGame
  (Utilities|FlowControl|Delay 1.0)
  (Game|OpenLevel(byObjectReference) "/Game/Logic/Maps/EndGameMap.EndGameMap"))

(event EventBeginPlay
  (|CallParentFunction) ; This node is disabled and will not be called.\nDrag off pins to build functionality.
)

(event Collision|EventActorBeginOverlap
  (params (OtherActor :type Actor%20Object%20Reference))
  (|CallParentFunction OtherActor) ; This node is disabled and will not be called.\nDrag off pins to build functionality.
)

(event EventTick
  (params (DeltaSeconds :type Float%20%28single-precision%29))
  (|CallParentFunction DeltaSeconds) ; This node is disabled and will not be called.\nDrag off pins to build functionality.
)

(event EventInteract
  (CallFunction|GetPlayerAcorns))

(fn ConstructionScript
  (|CallParentFunction))

(fn GetPlayerAcorns
  (bind _bp_inventorycomponent (Variables|Default|GetBP_InventoryComponent))
  (bind _output_get (LocalVariables|SetPlayer (Variables|/Game/Logic/Blueprints/Core/BP_TopDownGameMode.BP_TopDownGameMode_C|GetPlayer (.AsBP%20Top%20Down%20Game%20Mode (Utilities|Casting|CastToBP_TopDownGameMode (Game|GetGameMode))))))
  (bind _totalremoved (Default|RemoveAllItemsOfType (Variables|/Game/Logic/Blueprints/Character/BP_TopDownCharacter.BP_TopDownCharacter_C|GetInventory%20Component _output_get) "NewEnumerator0"))
  (bind _output_get_2 (LocalVariables|SetAcornsGotFromPlayer _totalremoved))
  (Utilities|FlowControl|Sequence
    (:then_0
      (if (not (> _output_get_2 0))
        (CallFunction|ShowBubble)))
    (:then_1
      (for _index (range 0 (- _output_get_2 1))
        (Default|AddtoInventory _bp_inventorycomponent "NewEnumerator0"))
      (if (Default|IsInventoryFull _bp_inventorycomponent)
        (Default|FadeOut (LocalVariables|GetPlayer))
        (CallFunction|EndGame)))))