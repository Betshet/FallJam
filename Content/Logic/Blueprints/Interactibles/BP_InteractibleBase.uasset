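; Base Blueprint for interactible objects, showing an interaction prompt while the top-down character is nearby.
; InteractSphere overlap events toggle the InteractionPrompt's visibility, reacting only to BP_TopDownCharacter.
; The Interact event is a placeholder that only prints a debug message, and nothing in this graph calls it.
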(event OnComponentBeginOverlap(InteractSphere)
  (params (OverlappedComponent :type Primitive%20Component%20Object%20Reference) (OtherActor :type Actor%20Object%20Reference) (OtherComp :type Primitive%20Component%20Object%20Reference) (OtherBodyIndex :type Integer) (bFromSweep :type Boolean) (SweepResult :type Hit%20Result%20Structure%20%28by%20ref%29))
  (if (Class|GameplayStatics|ObjectIsA OtherActor "/Game/Logic/Blueprints/Character/BP_TopDownCharacter.BP_TopDownCharacter_C")
    (Rendering|SetVisibility (Variables|Default|GetInteractionPrompt) true false)))

(event OnComponentEndOverlap(InteractSphere)
  (params (OverlappedComponent :type Primitive%20Component%20Object%20Reference) (OtherActor :type Actor%20Object%20Reference) (OtherComp :type Primitive%20Component%20Object%20Reference) (OtherBodyIndex :type Integer))
  (if (Class|GameplayStatics|ObjectIsA OtherActor "/Game/Logic/Blueprints/Character/BP_TopDownCharacter.BP_TopDownCharacter_C")
    (Rendering|SetVisibility (Variables|Default|GetInteractionPrompt) false false)))

(event EventInteract
  (Development|PrintString "I got interacted with"))

(fn ConstructionScript)